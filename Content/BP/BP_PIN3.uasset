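; BP_PIN3 is a pin actor that slides along world negative X after its open event (핀3열림) sets a negative step.
; While the move flag (핀3이동) is true, Tick applies that frame-rate-dependent offset and clears the flag at an X limit.
; While the flag is false, Tick calls the stop event (핀3멈춤), which zeroes the step and broadcasts 핀3멈춤정보 through a DoOnce.
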(event `self.ReceiveTick`
  (params (DeltaSeconds :type "Float (single-precision)"))
  (bind _returnvalue_x (`KismetMathLibrary.BreakVector` (`self.K2_GetActorLocation`)))
  (if (`self.핀3 이동`)
    (`self.K2_AddActorWorldOffset` (`KismetMathLibrary.MakeVector` (`self.Delta Location X`)))
    (if (<= _returnvalue_x -500.0)
      (set `self.핀3 이동` false))
    (else
      (`self.핀3멈춤`))))

(event `핀3열림`
  (set `self.Delta Location X` -3.0))

(event `핀3멈춤`
  (set `self.Delta Location X` 0.0)
  (`/Engine/EditorBlueprintResources/StandardMacros.DoOnce` false
    (:`Completed`
      (`self.핀3멈춤정보`))))

(fn `UserConstructionScript`)