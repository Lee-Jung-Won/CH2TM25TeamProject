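; BP_Sphere is a sphere actor that moves along world Y and announces when it stops.
; While the 스페어이동 (move) flag is true, Tick offsets it by DeltaLocationY each frame, without delta-time scaling.
; The 스패어이동 event sets that step but not the flag.
; When the flag is false, 스페어멈춤 (stop) uses DoOnce, never reset, to zero the step and call the 스페어멈춤정보 (stop info) dispatcher.
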(event `self.ReceiveBeginPlay`)

(event `self.ReceiveTick`
  (params (DeltaSeconds :type "Float (single-precision)"))
  (if (`self.스페어 이동`)
    (`self.K2_AddActorWorldOffset` (`KismetMathLibrary.MakeVector` 0.0 (`self.Delta Location Y`)))
    (else
      (`self.스페어 멈춤`))))

(event `스패어 이동`
  (set `self.Delta Location Y` 3.0))

(event `스페어 멈춤`
  (`/Engine/EditorBlueprintResources/StandardMacros.DoOnce` false
    (:`Completed`
      (set `self.Delta Location Y` 0.0)
      (`self.스페어 멈춤 정보`))))

(fn `UserConstructionScript`)