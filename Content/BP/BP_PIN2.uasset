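; BP_PIN2 is an actor for "pin 2" that slides along world X, with open, stop and close events setting its per-tick step.
; While the 핀2이동 (move) flag is true, Tick applies that step and clears the flag at the X limit.
; Otherwise Tick calls stop, then close near or below that limit, but applies no offset.
; Nothing here calls open or sets the flag true.
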(event `self.ReceiveTick`
  (params (DeltaSeconds :type "Float (single-precision)"))
  (bind _returnvalue_x (`KismetMathLibrary.BreakVector` (`self.K2_GetActorLocation`)))
  (bind _returnvalue_x_2 (`KismetMathLibrary.BreakVector` (`self.K2_GetActorLocation`)))
  (if (`self.핀2 이동`)
    (`self.K2_AddActorWorldOffset` (`KismetMathLibrary.MakeVector` (`self.Delta Location X`)))
    (if (>= _returnvalue_x_2 500.0)
      (set `self.핀2 이동` false))
    (else
      (`self.핀2멈춤`)
      (if (<= _returnvalue_x 501.0)
        (`self.핀2닫힘`)))))

(event `핀2열림`
  (set `self.Delta Location X` 3.0))

(event `핀2멈춤`
  (set `self.Delta Location X` 0.0))

(event `핀2닫힘`
  (set `self.Delta Location X` -3.0))

(fn `UserConstructionScript`)