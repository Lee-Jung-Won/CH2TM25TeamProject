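; BP_PIN is the first pin in a moving-pin chain, rising vertically and then triggering the next pins.
; 핀1이동 sets the per-tick Z offset, which Tick applies while its flag is true, without delta-time scaling.
; At the height threshold, Tick calls 핀1멈춤 and starts BP_PIN2 and BP_PIN3 from BPPINS, repeating each qualifying tick.
; DoOnce gates make the start and stop dispatchers fire only once.
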(event `self.ReceiveTick`
  (params (DeltaSeconds :type "Float (single-precision)"))
  (bind (_returnvalue_x _returnvalue_y _returnvalue_z) (`KismetMathLibrary.BreakVector` (`self.K2_GetActorLocation`)))
  (if (`self.핀1이동`)
    (`self.K2_AddActorWorldOffset` (`KismetMathLibrary.MakeVector` 0.0 0.0 (`self.Delta Location Z`)))
    (if (>= _returnvalue_z 500.0)
      (`self.핀1 멈춤`)
      (for _array_element (`self.BP_PINS`)
        (bind _asbp_pin2 (cast `/Game/BP/BP_PIN2` _array_element)
          (:`then`
            (`/Game/BP/BP_PIN2.핀2이동` _asbp_pin2))
          (:`CastFailed`
            (bind _asbp_pin3 (cast `/Game/BP/BP_PIN3` _array_element))
            (`/Game/BP/BP_PIN3.핀3이동` _asbp_pin3)))))))

(event `핀1 이동`
  (`/Engine/EditorBlueprintResources/StandardMacros.DoOnce` false
    (:`Completed`
      (set `self.Delta Location Z` 3.0)
      (`self.핀1 이동 정보`))))

(event `핀1 멈춤`
  (set `self.Delta Location Z` 0.0)
  (`/Engine/EditorBlueprintResources/StandardMacros.DoOnce` false
    (:`Completed`
      (`self.핀1멈충정보`))))

(fn `UserConstructionScript`)